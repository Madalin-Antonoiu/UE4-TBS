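; Player controller that tracks the selected unit and relays movement paths to it.
; Selecting a new unit deselects the previous valid one, and a newly available path is forwarded to the current unit to move along.
; The R key uses a FlipFlop to alternately hide and show every BP_Base_Obstacle actor in the level.
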(event Custom|Event_NewUnitSelected
  (params (Unit :type BP%20Unit%20Object%20Reference))
  (Utilities|IsValid (Variables|Default|GetselectedUnit)
    (:Is%20Valid
      (Default|EventDeselected (Variables|Default|GetselectedUnit)))
    (:Is%20Not%20Valid
      _))
  (Variables|Default|SetselectedUnit Unit))

(event Custom|Event_NewPathAvailable
  (params (path :type Array%20of%20Vector%202D%20Structures))
  (Utilities|IsValid (Variables|Default|GetselectedUnit)
    (:Is%20Valid
      (Default|EventMoveUnitAlongthePath (Variables|Default|GetselectedUnit) path))))

(event Input|KeyboardEvents|R
  (params (Key :type Key%20Structure :default "None"))
  ;[1 1 1] How cool is this.. Press R hides the actors, press R again shows them. Basically toggle visibility of Obstacles
  (:Pressed
    (Utilities|FlowControl|FlipFlop
      (:A
        (bind _outactors (Actor|GetAllActorsOfClass "/Game/Blueprints/Obstacles/BP_Base_Obstacle.BP_Base_Obstacle_C"))
        (for _array_element _outactors
          (Rendering|SetActorHiddenInGame _array_element true)))
      (:B
        (bind _outactors_2 (Actor|GetAllActorsOfClass "/Game/Blueprints/Obstacles/BP_Base_Obstacle.BP_Base_Obstacle_C"))
        (for _array_element_2 _outactors_2
          (Rendering|SetActorHiddenInGame _array_element_2 false))))))

(fn ConstructionScript)