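; Selectable grid unit that snaps to the nearest BP_Grid tile on BeginPlay and gets a random cone color.
; Clicking its capsule or cones toggles selection through BP_PlayerController.
; Given a path, it claims the destination tile in the grid's tile map, then rebuilds the grid's shared spline.
; A timeline moves it along that spline, with play rate scaled by path length and the grid flagged busy until finished.
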(event OnClicked(CapsuleComponent)
  (params (TouchedComponent :type Primitive%20Component%20Object%20Reference) (ButtonPressed :type Key%20Structure :default "None"))
  (if (!= (Variables|/Game/Blueprints/Controllers/BP_PlayerController.BP_PlayerController_C|GetselectedUnit (Variables|Default|GetplayerController)) self)
    (Default|EventNewUnitSelected (Variables|Default|GetplayerController) self)
    (CallFunction|EventSelected)
    (else
      (Default|EventNewUnitSelected (Variables|Default|GetplayerController)))))

(event OnClicked(Cone1)
  (params (TouchedComponent :type Primitive%20Component%20Object%20Reference) (ButtonPressed :type Key%20Structure :default "None"))
  (if (!= (Variables|/Game/Blueprints/Controllers/BP_PlayerController.BP_PlayerController_C|GetselectedUnit (Variables|Default|GetplayerController)) self)
    (Default|EventNewUnitSelected (Variables|Default|GetplayerController) self)
    (CallFunction|EventSelected)
    (else
      (Default|EventNewUnitSelected (Variables|Default|GetplayerController)))))

(event OnClicked(Cone)
  (params (TouchedComponent :type Primitive%20Component%20Object%20Reference) (ButtonPressed :type Key%20Structure :default "None"))
  (if (!= (Variables|/Game/Blueprints/Controllers/BP_PlayerController.BP_PlayerController_C|GetselectedUnit (Variables|Default|GetplayerController)) self)
    (Default|EventNewUnitSelected (Variables|Default|GetplayerController) self)
    (CallFunction|EventSelected)
    (else
      (Default|EventNewUnitSelected (Variables|Default|GetplayerController)))))

(event Custom|Event_Deselected
  (Development|PrintString "Deselected"))

(event Custom|Event_Selected
  (Development|PrintString "Selected"))

(event Custom|Event_MoveUnitAlongThePath
  (params (path :type Array%20of%20Vector%202D%20Structures))
  (Variables|Default|Setpath path)
  ;[1 1 1 1 14] remember my last clicked index :)
  (Utilities|Array|Insert (Variables|Default|Getpath) (Variables|Default|GetgridIndex))
  (CallFunction|UnitonThisTile (Utilities|Array|Get(acopy) (Variables|Default|Getpath) (Utilities|Array|LastIndex (Variables|Default|Getpath))))
  (Spline|ClearSplinePoints (Variables|/Game/Blueprints/BP_Grid.BP_Grid_C|GetSpline (Variables|Default|Getgrid)) true)
  (for _array_element (Variables|Default|Getpath)
    (Spline|AddSplinePoint (Variables|/Game/Blueprints/BP_Grid.BP_Grid_C|GetSpline (Variables|Default|Getgrid)) (Math|Vector|MakeVector (.x (.worldlocation (.Value (Utilities|Map|Find (Variables|/Game/Blueprints/BP_Grid.BP_Grid_C|Getstruct_Tiles (Variables|Default|Getgrid)) _array_element)))) (.y (.worldlocation (.Value (Utilities|Map|Find (Variables|/Game/Blueprints/BP_Grid.BP_Grid_C|Getstruct_Tiles (Variables|Default|Getgrid)) _array_element)))) (+ (.z (.worldlocation (.Value (Utilities|Map|Find (Variables|/Game/Blueprints/BP_Grid.BP_Grid_C|Getstruct_Tiles (Variables|Default|Getgrid)) _array_element)))) (Variables|/Script/Engine.CapsuleComponent|GetCapsuleHalfHeight (Variables|Collision|GetCapsuleComponent)))) "World" true))
  (Variables|/Game/Blueprints/BP_Grid.BP_Grid_C|SetbIsAUnitMoving (Variables|Default|Getgrid) true)
  ;[1 1 1 1 12] Same travel time duration  for unit travelling 2 tiles or 15 tiles for e.g
  (Components|Timeline|SetPlayRate (Variables|Default|GetMoveAlongThePathTimeline) (/ 1.0 (* (Utilities|Array|Length (Variables|Default|Getpath)) 0.2)))
  ;[1 1 1 1 14] Start Moving <#
  (bind _movementprogression (Timeline|MoveAlongThePathTimeline PlayFromStart)
    (:Update
      (Transformation|SetActorTransform self (Math|Transform|MakeTransform (Spline|GetLocationatDistanceAlongSpline (Variables|/Game/Blueprints/BP_Grid.BP_Grid_C|GetSpline (Variables|Default|Getgrid)) (* _movementprogression (Spline|GetSplineLength (Variables|/Game/Blueprints/BP_Grid.BP_Grid_C|GetSpline (Variables|Default|Getgrid)))) "World") (Spline|GetRotationatDistanceAlongSpline (Variables|/Game/Blueprints/BP_Grid.BP_Grid_C|GetSpline (Variables|Default|Getgrid)) (* _movementprogression (Spline|GetSplineLength (Variables|/Game/Blueprints/BP_Grid.BP_Grid_C|GetSpline (Variables|Default|Getgrid)))) "World") "1,1,1")))
    (:Finished
      (Variables|/Game/Blueprints/BP_Grid.BP_Grid_C|SetbIsAUnitMoving (Variables|Default|Getgrid) false))))

(event EventBeginPlay
  (Utilities|FlowControl|Delay 0.1)
  (Variables|Default|SetplayerController (.AsBP%20Player%20Controller (Utilities|Casting|CastToBP_PlayerController (Game|GetPlayerController 0))))
  (bind _outactors (Actor|GetAllActorsOfClass "/Game/Blueprints/BP_Grid.BP_Grid_C"))
  (Variables|Default|Setgrid (Utilities|Array|Get(acopy) _outactors))
  (CallFunction|SetGridIndexandSnaptoLocation)
  ;[1 1 1] Set random unit cone colors on play to differentiate them
  (bind _output_get (Variables|UnitProperties|SetunitColor (Utilities|Struct|MakeLinearColor (Math|Random|RandomFloatinRange 0.0 1.0) (Math|Random|RandomFloatinRange 0.0 1.0) (Math|Random|RandomFloatinRange 0.0 1.0) 1.0)))
  (Rendering|Material|SetVectorParameterValueonMaterials (Variables|Default|GetCone) "TileColor" (Math|Conversions|ToVector(LinearColor) _output_get)))

(fn ConstructionScript)

(fn SetGridIndexandSnaptoLocation
  (LocalVariables|SetclosestDistance 9999999.0)
  (bind _keys (Utilities|Map|Keys (Variables|/Game/Blueprints/BP_Grid.BP_Grid_C|Getstruct_Tiles (Variables|Default|Getgrid))))
  (for _array_element _keys
    (if (< (Math|Vector|VectorLength (- (.worldlocation (.Value (Utilities|Map|Find (Variables|/Game/Blueprints/BP_Grid.BP_Grid_C|Getstruct_Tiles (Variables|Default|Getgrid)) _array_element))) (Transformation|GetActorLocation self))) (LocalVariables|GetclosestDistance))
      (LocalVariables|SetclosestDistance (Math|Vector|VectorLength (- (.worldlocation (.Value (Utilities|Map|Find (Variables|/Game/Blueprints/BP_Grid.BP_Grid_C|Getstruct_Tiles (Variables|Default|Getgrid)) _array_element))) (Transformation|GetActorLocation self))))
      (LocalVariables|SetclosestIndex _array_element)))
  (CallFunction|UnitonThisTile (LocalVariables|GetclosestIndex))
  (Transformation|SetActorLocation (.worldlocation (.Value (Utilities|Map|Find (Variables|/Game/Blueprints/BP_Grid.BP_Grid_C|Getstruct_Tiles (Variables|Default|Getgrid)) (LocalVariables|GetclosestIndex)))) false false))

(fn UnitonThisTile
  (params (gridIndex :type Vector%202D%20Structure))
  (Utilities|Map|Add (Variables|/Game/Blueprints/BP_Grid.BP_Grid_C|Getstruct_Tiles (Variables|Default|Getgrid)) (Variables|Default|GetgridIndex) (Utilities|Struct|MakeStruct_Tiles (.tileactor (.Value (Utilities|Map|Find (Variables|/Game/Blueprints/BP_Grid.BP_Grid_C|Getstruct_Tiles (Variables|Default|Getgrid)) (Variables|Default|GetgridIndex)))) 0 (.groundtype (.Value (Utilities|Map|Find (Variables|/Game/Blueprints/BP_Grid.BP_Grid_C|Getstruct_Tiles (Variables|Default|Getgrid)) (Variables|Default|GetgridIndex)))) (.worldlocation (.Value (Utilities|Map|Find (Variables|/Game/Blueprints/BP_Grid.BP_Grid_C|Getstruct_Tiles (Variables|Default|Getgrid)) (Variables|Default|GetgridIndex)))) (.gridindex (.Value (Utilities|Map|Find (Variables|/Game/Blueprints/BP_Grid.BP_Grid_C|Getstruct_Tiles (Variables|Default|Getgrid)) (Variables|Default|GetgridIndex)))) (.tilecost (.Value (Utilities|Map|Find (Variables|/Game/Blueprints/BP_Grid.BP_Grid_C|Getstruct_Tiles (Variables|Default|Getgrid)) (Variables|Default|GetgridIndex)))) (.finalcost (.Value (Utilities|Map|Find (Variables|/Game/Blueprints/BP_Grid.BP_Grid_C|Getstruct_Tiles (Variables|Default|Getgrid)) (Variables|Default|GetgridIndex)))) (.costfromstart (.Value (Utilities|Map|Find (Variables|/Game/Blueprints/BP_Grid.BP_Grid_C|Getstruct_Tiles (Variables|Default|Getgrid)) (Variables|Default|GetgridIndex)))) (.estimatedcosttotarget (.Value (Utilities|Map|Find (Variables|/Game/Blueprints/BP_Grid.BP_Grid_C|Getstruct_Tiles (Variables|Default|Getgrid)) (Variables|Default|GetgridIndex)))) (.previoustile (.Value (Utilities|Map|Find (Variables|/Game/Blueprints/BP_Grid.BP_Grid_C|Getstruct_Tiles (Variables|Default|Getgrid)) (Variables|Default|GetgridIndex))))))
  (Variables|Default|SetgridIndex gridIndex)
  (Utilities|Map|Add (Variables|/Game/Blueprints/BP_Grid.BP_Grid_C|Getstruct_Tiles (Variables|Default|Getgrid)) (Variables|Default|GetgridIndex) (Utilities|Struct|MakeStruct_Tiles (.tileactor (.Value (Utilities|Map|Find (Variables|/Game/Blueprints/BP_Grid.BP_Grid_C|Getstruct_Tiles (Variables|Default|Getgrid)) (Variables|Default|GetgridIndex)))) self (.groundtype (.Value (Utilities|Map|Find (Variables|/Game/Blueprints/BP_Grid.BP_Grid_C|Getstruct_Tiles (Variables|Default|Getgrid)) (Variables|Default|GetgridIndex)))) (.worldlocation (.Value (Utilities|Map|Find (Variables|/Game/Blueprints/BP_Grid.BP_Grid_C|Getstruct_Tiles (Variables|Default|Getgrid)) (Variables|Default|GetgridIndex)))) (.gridindex (.Value (Utilities|Map|Find (Variables|/Game/Blueprints/BP_Grid.BP_Grid_C|Getstruct_Tiles (Variables|Default|Getgrid)) (Variables|Default|GetgridIndex)))) (.tilecost (.Value (Utilities|Map|Find (Variables|/Game/Blueprints/BP_Grid.BP_Grid_C|Getstruct_Tiles (Variables|Default|Getgrid)) (Variables|Default|GetgridIndex)))) (.finalcost (.Value (Utilities|Map|Find (Variables|/Game/Blueprints/BP_Grid.BP_Grid_C|Getstruct_Tiles (Variables|Default|Getgrid)) (Variables|Default|GetgridIndex)))) (.costfromstart (.Value (Utilities|Map|Find (Variables|/Game/Blueprints/BP_Grid.BP_Grid_C|Getstruct_Tiles (Variables|Default|Getgrid)) (Variables|Default|GetgridIndex)))) (.estimatedcosttotarget (.Value (Utilities|Map|Find (Variables|/Game/Blueprints/BP_Grid.BP_Grid_C|Getstruct_Tiles (Variables|Default|Getgrid)) (Variables|Default|GetgridIndex)))) (.previoustile (.Value (Utilities|Map|Find (Variables|/Game/Blueprints/BP_Grid.BP_Grid_C|Getstruct_Tiles (Variables|Default|Getgrid)) (Variables|Default|GetgridIndex)))))))