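; BP_GameMode is the game mode that sets up the turn-based combat screen when play begins.
; On BeginPlay it creates a W_CombatScreenTurns widget, stores it and adds it to the player screen.
; It then finds the first BP_Grid and all BP_Unit actors in the level and passes them, along with the BP_PlayerController, into the widget's variables.
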(event EventBeginPlay
  (bind _returnvalue (UserInterface|CreateWidget "/Game/Blueprints/UI/W_CombatScreenTurns.W_CombatScreenTurns_C"))
  (bind _output_get (Variables|Default|SetNext%20Turn%20Combat%20Screen _returnvalue))
  (UserInterface|Viewport|AddtoPlayerScreen _output_get)
  ;[1 1 1] how to pass a variable over to combat screen
  (bind _outactors (Actor|GetAllActorsOfClass "/Game/Blueprints/Grid/BP_Grid.BP_Grid_C"))
  (bind _output_get_2 (Variables|Default|Setgrid (Utilities|Array|Get(acopy) _outactors)))
  (Variables|/Game/Blueprints/UI/W_CombatScreenTurns.W_CombatScreenTurns_C|Setgrid (Variables|Default|GetNext%20Turn%20Combat%20Screen) _output_get_2)
  ;[1 1 1] Writting values into Unit List
  (bind _outactors_2 (Actor|GetAllActorsOfClass "/Game/Blueprints/Controllers/BP_Unit.BP_Unit_C"))
  (Variables|/Game/Blueprints/UI/W_CombatScreenTurns.W_CombatScreenTurns_C|SetunitList (Variables|Default|GetNext%20Turn%20Combat%20Screen) _outactors_2)
  (Variables|/Game/Blueprints/UI/W_CombatScreenTurns.W_CombatScreenTurns_C|SetplayerController (Variables|Default|GetNext%20Turn%20Combat%20Screen) (.AsBP%20Player%20Controller (Utilities|Casting|CastToBP_PlayerController (Game|GetPlayerController 0)))))

(fn ConstructionScript)