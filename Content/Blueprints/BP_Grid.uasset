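; Grid manager for tactical unit movement that builds tiles from the level and handles tile selection, hover and path highlighting.
; Sphere traces for ground and obstacles fill a tile map with ground type and cost, debug-drawn on construction and spawned as BP_GridTile actors at BeginPlay.
; Hovering runs four-way, A*-style pathfinding within the selected unit's movement points, skipping occupied and impassable tiles.
; The same search's closed set supplies reachable tiles.
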(event Custom|Event_NewTileSelected
  (params (selectedTile :type BP%20Grid%20Tile%20Object%20Reference))
  ;[1 1 1 1 14] Deselect Tile after new selection is made <3
  (Utilities|IsValid (Variables|Grid|GetselectedTile)
    (:Is%20Valid
      (Default|EventDeselectTile (Variables|Grid|GetselectedTile)))
    (:Is%20Not%20Valid
      _))
  (Variables|Grid|SetselectedTile selectedTile)
  ;[1 1 1] Allow pathfinding calculation only if Unit not moving
  (if (not (Variables|UnitsMovement|GetbIsAUnitMoving))
    (Default|EventNewPathAvailable (Variables|UnitsMovement|GetplayerController) (Variables|Pathfinding|Getpath))))

(event Custom|Event_NewTileMouseOver
  (params (HoveredTile :type BP%20Grid%20Tile%20Object%20Reference))
  (bind _playercontroller (Variables|UnitsMovement|GetplayerController))
  (bind _selectedunit (Variables|/Game/Blueprints/Controllers/BP_PlayerController.BP_PlayerController_C|GetselectedUnit _playercontroller))
  ;[1 1 1 1 14] Highlight tile on HOVER
  (Utilities|IsValid (Variables|Grid|GethoveredTile)
    (:Is%20Valid
      (Default|EventEndHoverTile (Variables|Grid|GethoveredTile)))
    (:Is%20Not%20Valid
      _))
  (Variables|Grid|SethoveredTile HoveredTile)
  ;[1 1 1] Highlight current path on Hover
  ;;[1 1 1] Needed for retrace
  (Pathfinding|HighlightCurrentPath false)
  (if (Math|Boolean|ANDBoolean (Utilities|IsValid _selectedunit) (Utilities|IsValid (Variables|Grid|GethoveredTile)) (not (Variables|UnitsMovement|GetbIsAUnitMoving)))
    (Pathfinding|FindPathtoTarget (Variables|/Game/Blueprints/Controllers/BP_Unit.BP_Unit_C|GetgridIndex _selectedunit) (Variables|/Game/Blueprints/Tile/BP_GridTile.BP_GridTile_C|GetgridIndex (Variables|Grid|GethoveredTile)) false)
    (Pathfinding|HighlightCurrentPath true)))

(event EventBeginPlay
  ;[1 1 1] Generate Map Data and Spawn Tiles
  (Variables|Grid|SetGridLocation (Transformation|GetWorldLocation (Variables|Default|GetScene)))
  (Grid|GenerateMapDatafromWorld)
  (Grid|SpawnTile false)
  ;[1 1 1 1 14] Set the active player controller as NO selection
  (Variables|UnitsMovement|SetplayerController (.AsBP%20Player%20Controller (Utilities|Casting|CastToBP_PlayerController (Game|GetPlayerController 0)))))

(fn ConstructionScript
  (bind _gridsizeworld (Variables|Grid|GetGridSizeWorld))
  ;[1 1 1 1 14] Setting Grid World Location at Runtime ( no need to drop anything in the scene then) #1
  (Rendering|Debug|FlushPersistentDebugLines)
  (Variables|Grid|SetGridLocation (Transformation|GetWorldLocation (Variables|Default|GetScene)))
  ;[1 1 1 1 14] Debug the grid outlines ( draw so it is visible) #2
  (Rendering|Debug|DrawDebugBox (Variables|Grid|GetGridLocation) (Math|Vector|MakeVector (.y _gridsizeworld) (.x _gridsizeworld) 5.0) (Variables|Debug|GetGridBoxColor) "0, 0, 0" 1e+03 1e+01)
  ;[1 1 1 1 14] Debug bottom left corner starting point #3 (GridBottomLeft needs to be created first)
  (Rendering|Debug|DrawDebugBox (Grid|GridBottomLeft) (Math|Vector|MakeVector 2e+01 2e+01 2e+01) (Variables|Debug|GetBottomLeftColor) "0, 0, 0" 1e+03 1e+01)
  ;[1 1 1 1 14] Generate map data, #4
  (Grid|GenerateMapDatafromWorld)
  ;[1 1 1 1 14] Draw the Tiles #5(create DrawTile function beforehand)
  (Debug|DrawTile))

(fn GridBottomLeft
  (bind _scene (Variables|Default|GetScene))
  ;[1 1 1 1 14] (Grid Location - ( Scene.GetRightVector * GridSizeX)) - Scene.GetForwardVector * GridSizeY = GridBottomLeft
  (return (- (- (Variables|Grid|GetGridLocation) (* (Math|Vector|GetRightVector _scene) (.x (Variables|Grid|GetGridSizeWorld)))) (* (Math|Vector|GetForwardVector _scene) (.y (Variables|Grid|GetGridSizeWorld))))))

(fn GridTileNumber
  (bind _gridsizeworld (Variables|Grid|GetGridSizeWorld))
  (bind _tilesize (Variables|Grid|GetTileSize))
  (bind _returnvalue (/ _gridsizeworld _tilesize))
  ;[1 1 1 1 14] GridSizeWorld / TileSize. Return (X rounded -1 , Y rounded -1)
  (return (- (Math|Float|Round (.x _returnvalue)) 1) (- (Math|Float|Round (.y _returnvalue)) 1)))

(fn DrawTile
  (bind _keys (Utilities|Map|Keys (Variables|Grid|Getstruct_Tiles)))
  (for _array_element _keys
    (Debug|MyDrawDebugPlane (.worldlocation (.Value (Utilities|Map|Find (Variables|Grid|Getstruct_Tiles) _array_element))) (.groundtype (.Value (Utilities|Map|Find (Variables|Grid|Getstruct_Tiles) _array_element))))))

(fn MySphereTrace
  (params (Location :type Vector) (TraceChannel :type ETraceTypeQuery%20Enum :default "TraceTypeQuery1"))
  ;[1 1 1] Generate tracing Spheres on tiles hit
  (bind (_outhit _returnvalue) (Collision|SphereTraceByChannel Location Location (- (Variables|Grid|GetTileSize) (Variables|Grid|GetTileGapSize)) TraceChannel false 0 (Variables|Debug|GetDraw%20Debug%20Spheres) true "(R=1.000000,G=0.000000,B=0.000000,A=1.000000)" "(R=0.000000,G=1.000000,B=0.000000,A=1.000000)" 2e+01))
  (return (.hitactor _outhit) _returnvalue))

(fn MyDrawDebugPlane
  (params (Location :type Vector) (GroundType :type Enum_GroundTypes%20Enum :default "NewEnumerator0"))
  (switch Utilities|FlowControl|Switch|SwitchonEnum_GroundTypes GroundType
    (:NewEnumerator0
      (LocalVariables|SetTileColor "(R=0.508662,G=0.541667,B=0.476215,A=1.000000)"))
    (:NewEnumerator1
      (LocalVariables|SetTileColor "(R=0.963542,G=0.895448,B=0.124347,A=1.000000)"))
    (:NewEnumerator2
      (LocalVariables|SetTileColor "(R=0.562500,G=0.174123,B=0.056585,A=1.000000)"))
    (:NewEnumerator3
      (LocalVariables|SetTileColor "(R=0.933333,G=0.000000,B=0.040256,A=1.000000)")))
  (Class|KismetSystemLibrary|DrawDebugPlane (Utilities|Struct|MakePlane (.Z (Math|Vector|BreakVector Location)) 0.0 0.0 1.0) Location (- (Variables|Grid|GetTileSize) (Variables|Grid|GetTileGapSize)) (LocalVariables|GetTileColor) 1e+06))

(fn GenerateMapDatafromWorld
  (bind (_gridtilenumberx _gridtilenumbery) (Grid|GridTileNumber))
  (bind _tilesize (Variables|Grid|GetTileSize))
  (bind _tilesize_2 (Variables|Grid|GetTileSize))
  ;[1 1 1 1 14] for x number of tiles, and y number of tiles, x[i] =x , y[j] =y locally saved variables   #part1
  (for _index (range 0 _gridtilenumberx)
    (LocalVariables|SetX _index)
    (for _index_2 (range 0 _gridtilenumbery)
      (LocalVariables|SetY _index_2)
      ;[1 1 1] TilePosition = GridBottomLeft + ( Scene.Right * TileSize) + (Scene.Forward *TileSize), #part2
      ; So it draws a square starting from bottom left position.
      (LocalVariables|SetTilePosition (+ (Grid|GridBottomLeft) (* (Math|Vector|GetRightVector (Variables|Default|GetScene)) (+ (* (LocalVariables|GetX) (* _tilesize_2 2.0)) _tilesize_2)) (* (Math|Vector|GetForwardVector (Variables|Default|GetScene)) (+ (* (LocalVariables|GetY) (* _tilesize 2.0)) _tilesize))))
      ;[1 1 1 1 14] Sphere Trace Collision for GROUND, #part4
      (if (.HitSomething (Grid|MySphereTrace (LocalVariables|GetTilePosition) "TraceTypeQuery3"))
        ;[1 1 1 1 14] Sphere Trace Collision for OBSTACLES, #part5
        (if (.HitSomething (Grid|MySphereTrace (LocalVariables|GetTilePosition) "TraceTypeQuery4"))
          ;[1 1 1] If tiles HIT an obstacle
          (Utilities|Map|Add (Variables|Grid|Getstruct_Tiles) (Math|Vector2D|MakeVector2D (Math|Conversions|ToFloat(Integer) (LocalVariables|GetX)) (Math|Conversions|ToFloat(Integer) (LocalVariables|GetY))) (Utilities|Struct|MakeStruct_Tiles 0 0 (Variables|/Game/Blueprints/Obstacles/BP_Base_Obstacle.BP_Base_Obstacle_C|GetEnum_GroundTypes (.AsBP%20Base%20Obstacle (Utilities|Casting|CastToBP_Base_Obstacle (.Actor (Grid|MySphereTrace (LocalVariables|GetTilePosition) "TraceTypeQuery4"))))) (LocalVariables|GetTilePosition) (Math|Vector2D|MakeVector2D (Math|Conversions|ToFloat(Integer) (LocalVariables|GetX)) (Math|Conversions|ToFloat(Integer) (LocalVariables|GetY))) (Pathfinding|GetTileCost (Variables|/Game/Blueprints/Obstacles/BP_Base_Obstacle.BP_Base_Obstacle_C|GetEnum_GroundTypes (.AsBP%20Base%20Obstacle (Utilities|Casting|CastToBP_Base_Obstacle (.Actor (Grid|MySphereTrace (LocalVariables|GetTilePosition) "TraceTypeQuery4")))))) 0 0 0 "(X=0.000000,Y=0.000000)"))
          (else
            ;[1 1 1] If tiles didn't hit and obstacle, mark them as normal
            (Utilities|Map|Add (Variables|Grid|Getstruct_Tiles) (Math|Vector2D|MakeVector2D (Math|Conversions|ToFloat(Integer) (LocalVariables|GetX)) (Math|Conversions|ToFloat(Integer) (LocalVariables|GetY))) (Utilities|Struct|MakeStruct_Tiles 0 0 "NewEnumerator0" (LocalVariables|GetTilePosition) (Math|Vector2D|MakeVector2D (Math|Conversions|ToFloat(Integer) (LocalVariables|GetX)) (Math|Conversions|ToFloat(Integer) (LocalVariables|GetY))) (Pathfinding|GetTileCost "NewEnumerator0") 0 0 0 "(X=0.000000,Y=0.000000)"))))
        (else
          ;[1 1 1] if spheres don't hit the Ground, mark those tiles as NONE existent :)
          (Utilities|Map|Add (Variables|Grid|Getstruct_Tiles) (Math|Vector2D|MakeVector2D (Math|Conversions|ToFloat(Integer) (LocalVariables|GetX)) (Math|Conversions|ToFloat(Integer) (LocalVariables|GetY))) (Utilities|Struct|MakeStruct_Tiles 0 0 "NewEnumerator4" (LocalVariables|GetTilePosition) (Math|Vector2D|MakeVector2D (Math|Conversions|ToFloat(Integer) (LocalVariables|GetX)) (Math|Conversions|ToFloat(Integer) (LocalVariables|GetY))) (Pathfinding|GetTileCost "NewEnumerator4") 0 0 0 "(X=0.000000,Y=0.000000)")))))))

(fn SpawnTile
  (params (SpawnNoneTile :type Boolean))
  (Utilities|Array|Clear (Variables|Default|GetcurrentGridTiles))
  (bind _keys (Utilities|Map|Keys (Variables|Grid|Getstruct_Tiles)))
  (for _array_element _keys
    (if (or (Utilities|Enum|NotEqual(Enum) (.groundtype (.Value (Utilities|Map|Find (Variables|Grid|Getstruct_Tiles) _array_element))) "NewEnumerator4") SpawnNoneTile)
      (bind _returnvalue (Game|SpawnActorfromClass "/Game/Blueprints/Tile/BP_GridTile.BP_GridTile_C" (Math|Conversions|ToTransform(Vector) (.worldlocation (.Value (Utilities|Map|Find (Variables|Grid|Getstruct_Tiles) _array_element)))) "Undefined" 0 0))
      (Variables|/Game/Blueprints/Tile/BP_GridTile.BP_GridTile_C|SetgridIndex _returnvalue _array_element)
      (Variables|/Game/Blueprints/Tile/BP_GridTile.BP_GridTile_C|Setbp_Grid _returnvalue self)
      (Utilities|Map|Add (Variables|Grid|Getstruct_Tiles) _array_element (Utilities|Struct|MakeStruct_Tiles _returnvalue 0 (.groundtype (.Value (Utilities|Map|Find (Variables|Grid|Getstruct_Tiles) _array_element))) (.worldlocation (.Value (Utilities|Map|Find (Variables|Grid|Getstruct_Tiles) _array_element))) (.gridindex (.Value (Utilities|Map|Find (Variables|Grid|Getstruct_Tiles) _array_element))) (.tilecost (.Value (Utilities|Map|Find (Variables|Grid|Getstruct_Tiles) _array_element))) (.finalcost (.Value (Utilities|Map|Find (Variables|Grid|Getstruct_Tiles) _array_element))) (.costfromstart (.Value (Utilities|Map|Find (Variables|Grid|Getstruct_Tiles) _array_element))) (.estimatedcosttotarget (.Value (Utilities|Map|Find (Variables|Grid|Getstruct_Tiles) _array_element))) (.previoustile (.Value (Utilities|Map|Find (Variables|Grid|Getstruct_Tiles) _array_element)))))
      (Utilities|Array|AddUnique (Variables|Default|GetcurrentGridTiles) _returnvalue))))

(fn GetTileCost
  (params (gridIndex :type Enum_GroundTypes%20Enum :default "NewEnumerator0"))
  (switch Utilities|FlowControl|Switch|SwitchonEnum_GroundTypes gridIndex
    (:NewEnumerator0
      (LocalVariables|SetCost 1))
    (:NewEnumerator1
      (LocalVariables|SetCost 2))
    (:NewEnumerator2
      (LocalVariables|SetCost 5))
    (:NewEnumerator3
      (LocalVariables|SetCost 999 :!label _label))
    (:NewEnumerator4
      (goto _label)))
  (return (LocalVariables|GetCost)))

(fn GetTileNeighbours
  (params (gridIndex :type Vector%202D%20Structure))
  (bind _output_get (LocalVariables|SetpossibleNeighbours (Utilities|Array|MakeArray "(X=1.000000,Y=0.000000)" "(X=0.000000,Y=1.000000)" "(X=-1.000000,Y=0.000000)" "(X=0.000000,Y=-1.000000)")))
  (for _array_element _output_get
    (if (.ReturnValue (Utilities|Map|Find (Variables|Grid|Getstruct_Tiles) (+ _array_element gridIndex)))
      (if (Math|Boolean|ANDBoolean (Utilities|Enum|NotEqual(Enum) (.groundtype (.Value (Utilities|Map|Find (Variables|Grid|Getstruct_Tiles) (+ _array_element gridIndex)))) "NewEnumerator4") (Utilities|Enum|NotEqual(Enum) (.groundtype (.Value (Utilities|Map|Find (Variables|Grid|Getstruct_Tiles) (+ _array_element gridIndex)))) "NewEnumerator3") (== (.unitonthistile (.Value (Utilities|Map|Find (Variables|Grid|Getstruct_Tiles) (+ _array_element gridIndex)))) 0))
        (Utilities|Array|AddUnique (LocalVariables|GetoutNeighbours) (+ _array_element gridIndex)))))
  (return (LocalVariables|GetoutNeighbours)))

(fn GetEstimatedCosttoTarget
  (params (currentTile :type Vector%202D%20Structure) (targetTile :type Vector%202D%20Structure))
  (bind _returnvalue (- currentTile targetTile))
  (return (Math|Float|Round (+ (Math|Float|Absolute(Float) (.x _returnvalue)) (Math|Float|Absolute(Float) (.y _returnvalue))))))

(fn FindPathtoTarget
  (params (startTile :type Vector%202D%20Structure) (targetTile :type Vector%202D%20Structure) (bIsJustToFindReachables :type Boolean))
  (bind _struct_tiles (Variables|Grid|Getstruct_Tiles))
  (bind _struct_tiles_2 (Variables|Grid|Getstruct_Tiles))
  (bind _struct_tiles_3 (Variables|Grid|Getstruct_Tiles))
  (bind _struct_tiles_4 (Variables|Grid|Getstruct_Tiles))
  (LocalVariables|SetstartTileLocal startTile)
  (LocalVariables|SettargetTileLocal targetTile)
  (Utilities|Array|Clear (Variables|Pathfinding|Getpath))
  (if (or bIsJustToFindReachables (Math|Boolean|ANDBoolean (Utilities|Enum|NotEqual(Enum) (.groundtype (.Value (Utilities|Map|Find (Variables|Grid|Getstruct_Tiles) (LocalVariables|GettargetTileLocal)))) "NewEnumerator4") (Utilities|Enum|NotEqual(Enum) (.groundtype (.Value (Utilities|Map|Find (Variables|Grid|Getstruct_Tiles) (LocalVariables|GettargetTileLocal)))) "NewEnumerator3") (.ReturnValue (Utilities|Map|Find (Variables|Grid|Getstruct_Tiles) (LocalVariables|GettargetTileLocal))) (== (.unitonthistile (.Value (Utilities|Map|Find (Variables|Grid|Getstruct_Tiles) (LocalVariables|GettargetTileLocal)))) 0)))
    (Utilities|FlowControl|Sequence
      (:then_0
        ;[1 1 1] Default Values
        (bind _keys (Utilities|Map|Keys (Variables|Grid|Getstruct_Tiles)))
        (for _array_element _keys
          (Utilities|Map|Add _struct_tiles_4 _array_element (Utilities|Struct|MakeStruct_Tiles (.tileactor (.Value (Utilities|Map|Find _struct_tiles_4 _array_element))) (.unitonthistile (.Value (Utilities|Map|Find _struct_tiles_4 _array_element))) (.groundtype (.Value (Utilities|Map|Find _struct_tiles_4 _array_element))) (.worldlocation (.Value (Utilities|Map|Find _struct_tiles_4 _array_element))) (.gridindex (.Value (Utilities|Map|Find _struct_tiles_4 _array_element))) (.tilecost (.Value (Utilities|Map|Find _struct_tiles_4 _array_element))) 999 999 999 "(X=0.000000,Y=0.000000)")))
        (Utilities|Map|Add _struct_tiles (LocalVariables|GetstartTileLocal) (Utilities|Struct|MakeStruct_Tiles (.tileactor (.Value (Utilities|Map|Find _struct_tiles (LocalVariables|GetstartTileLocal)))) (.unitonthistile (.Value (Utilities|Map|Find _struct_tiles (LocalVariables|GetstartTileLocal)))) (.groundtype (.Value (Utilities|Map|Find _struct_tiles (LocalVariables|GetstartTileLocal)))) (.worldlocation (.Value (Utilities|Map|Find _struct_tiles (LocalVariables|GetstartTileLocal)))) (.gridindex (.Value (Utilities|Map|Find _struct_tiles (LocalVariables|GetstartTileLocal)))) (.tilecost (.Value (Utilities|Map|Find _struct_tiles (LocalVariables|GetstartTileLocal)))) (Pathfinding|GetEstimatedCosttoTarget (LocalVariables|GetstartTileLocal) (LocalVariables|GettargetTileLocal)) 0 (Pathfinding|GetEstimatedCosttoTarget (LocalVariables|GetstartTileLocal) (LocalVariables|GettargetTileLocal)) "(X=0.000000,Y=0.000000)")))
      (:then_1
        (LocalVariables|SetcurrentTile (LocalVariables|GetstartTileLocal))
        (Utilities|Array|AddUnique (LocalVariables|GetopenSet) (LocalVariables|GetstartTileLocal))
        (while (> (Utilities|Array|Length (LocalVariables|GetopenSet)) 0)
          (LocalVariables|SetopenSetCheapest (Utilities|Array|Get(acopy) (LocalVariables|GetopenSet)))
          (for _array_element_2 (LocalVariables|GetopenSet)
            (if (< (.finalcost (.Value (Utilities|Map|Find _struct_tiles_2 _array_element_2))) (.finalcost (.Value (Utilities|Map|Find _struct_tiles_2 (LocalVariables|GetopenSetCheapest)))))
              (LocalVariables|SetopenSetCheapest _array_element_2 :!label _label)
              (elif (== (.finalcost (.Value (Utilities|Map|Find _struct_tiles_2 _array_element_2))) (.finalcost (.Value (Utilities|Map|Find _struct_tiles_2 (LocalVariables|GetopenSetCheapest)))))
                (if (< (.estimatedcosttotarget (.Value (Utilities|Map|Find _struct_tiles_2 _array_element_2))) (.estimatedcosttotarget (.Value (Utilities|Map|Find _struct_tiles_2 (LocalVariables|GetopenSetCheapest)))))
                  (goto _label)))))
          (LocalVariables|SetcurrentTile (LocalVariables|GetopenSetCheapest))
          (Utilities|Array|RemoveItem (LocalVariables|GetopenSet) (LocalVariables|GetcurrentTile))
          (Utilities|Array|AddUnique (LocalVariables|GetclosedSet) (LocalVariables|GetcurrentTile))
          (for _array_element_3 (Pathfinding|GetTileNeighbours (LocalVariables|GetcurrentTile))
            (LocalVariables|SetcurrentNeighbour _array_element_3)
            (if (not (Utilities|Array|ContainsItem (LocalVariables|GetclosedSet) (LocalVariables|GetcurrentNeighbour)))
              (bind _output_get (LocalVariables|SetcurrentNeighbourCostFromStart (+ (.costfromstart (.Value (Utilities|Map|Find (Variables|Grid|Getstruct_Tiles) (LocalVariables|GetcurrentTile)))) (.tilecost (.Value (Utilities|Map|Find (Variables|Grid|Getstruct_Tiles) (LocalVariables|GetcurrentNeighbour)))))))
              (if (<= _output_get (Variables|/Game/Blueprints/Controllers/BP_Unit.BP_Unit_C|GetmovementPoints (Variables|/Game/Blueprints/Controllers/BP_PlayerController.BP_PlayerController_C|GetselectedUnit (Variables|UnitsMovement|GetplayerController))))
                (if (not (Utilities|Array|ContainsItem (LocalVariables|GetopenSet) (LocalVariables|GetcurrentNeighbour)))
                  (Utilities|Array|AddUnique (LocalVariables|GetopenSet) (LocalVariables|GetcurrentNeighbour))
                  (Utilities|Map|Add _struct_tiles_3 (LocalVariables|GetcurrentNeighbour) (Utilities|Struct|MakeStruct_Tiles (.tileactor (.Value (Utilities|Map|Find _struct_tiles_3 (LocalVariables|GetcurrentNeighbour)))) (.unitonthistile (.Value (Utilities|Map|Find _struct_tiles_3 (LocalVariables|GetcurrentNeighbour)))) (.groundtype (.Value (Utilities|Map|Find _struct_tiles_3 (LocalVariables|GetcurrentNeighbour)))) (.worldlocation (.Value (Utilities|Map|Find _struct_tiles_3 (LocalVariables|GetcurrentNeighbour)))) (.gridindex (.Value (Utilities|Map|Find _struct_tiles_3 (LocalVariables|GetcurrentNeighbour)))) (.tilecost (.Value (Utilities|Map|Find _struct_tiles_3 (LocalVariables|GetcurrentNeighbour)))) (+ (LocalVariables|GetcurrentNeighbourCostFromStart) (Pathfinding|GetEstimatedCosttoTarget (LocalVariables|GetcurrentNeighbour) (LocalVariables|GetstartTileLocal))) (LocalVariables|GetcurrentNeighbourCostFromStart) (Pathfinding|GetEstimatedCosttoTarget (LocalVariables|GetcurrentNeighbour) (LocalVariables|GetstartTileLocal)) (LocalVariables|GetcurrentTile)) :!label _label_2)
                  (if (Math|Vector|Equal(Vector) (LocalVariables|GetcurrentNeighbour) (LocalVariables|GettargetTileLocal) 0.0001)
                    (Variables|Pathfinding|Setpath (Pathfinding|RetracePath (LocalVariables|GettargetTileLocal) (LocalVariables|GetstartTileLocal)))
                    (return (LocalVariables|GetclosedSet)))
                  (elif (< (LocalVariables|GetcurrentNeighbourCostFromStart) (.costfromstart (.Value (Utilities|Map|Find _struct_tiles_3 (LocalVariables|GetcurrentNeighbour)))))
                    (goto _label_2)))))))
        ;[1 1 1 1 14] Fail
        (return (LocalVariables|GetclosedSet))))
    (else
      (return (LocalVariables|GetclosedSet)))))

(fn RetracePath
  (params (targetTile :type Vector%202D%20Structure) (startTile :type Vector%202D%20Structure))
  (LocalVariables|SetcurrentTile targetTile)
  (while (Math|Vector|NotEqual(Vector) (LocalVariables|GetcurrentTile) startTile 0.0001)
    (Utilities|Array|AddUnique (LocalVariables|GetinvertedPath) (LocalVariables|GetcurrentTile))
    (LocalVariables|SetcurrentTile (.previoustile (.Value (Utilities|Map|Find (Variables|Grid|Getstruct_Tiles) (LocalVariables|GetcurrentTile))))))
  (bind _arrayelement (Utilities|Array|ReverseforEachLoop (LocalVariables|GetinvertedPath))
    (:LoopBody
      (Utilities|Array|AddUnique (LocalVariables|GetoutPath) _arrayelement))
    (:Completed
      (return (LocalVariables|GetoutPath)))))

(fn HighlightCurrentPath
  (params (bIsForHighlight :type Boolean))
  (for _array_element (Variables|Pathfinding|Getpath)
    (Utilities|IsValid (.tileactor (.Value (Utilities|Map|Find (Variables|Grid|Getstruct_Tiles) _array_element)))
      (:Is%20Valid
        (Default|EventIsinPath (.tileactor (.Value (Utilities|Map|Find (Variables|Grid|Getstruct_Tiles) _array_element))) bIsForHighlight)))))

(fn HighlightReachableTiles
  (params (bIsForHighlight :type Boolean) (reachableIndexes :type Array%20of%20Vector%202D%20Structures))
  (for _array_element reachableIndexes
    (Utilities|IsValid (.tileactor (.Value (Utilities|Map|Find (Variables|Grid|Getstruct_Tiles) _array_element)))
      (:Is%20Valid
        (Default|EventIsReachable (.tileactor (.Value (Utilities|Map|Find (Variables|Grid|Getstruct_Tiles) _array_element))) bIsForHighlight)))))

(fn GetReachableTilesIndexes
  (params (startIndexes :type Vector%202D%20Structure) (movementPoints :type Integer))
  (LocalVariables|SetinStartIndex startIndexes)
  (LocalVariables|SetinMovementPoints movementPoints)
  (bind _keys (Utilities|Map|Keys (Variables|Grid|Getstruct_Tiles)))
  (bind _array_element (Utilities|Array|ForEachLoopwithBreak _keys :!label _label)
    (:LoopBody
      (LocalVariables|SettargetIndex _array_element)
      (if (Math|Boolean|ORBoolean (!= (.unitonthistile (.Value (Utilities|Map|Find (Variables|Grid|Getstruct_Tiles) (LocalVariables|GettargetIndex)))) 0) (Utilities|Enum|Equal(Enum) (.groundtype (.Value (Utilities|Map|Find (Variables|Grid|Getstruct_Tiles) (LocalVariables|GettargetIndex)))) "NewEnumerator3") (Utilities|Enum|Equal(Enum) (.groundtype (.Value (Utilities|Map|Find (Variables|Grid|Getstruct_Tiles) (LocalVariables|GettargetIndex)))) "NewEnumerator4") (> (Pathfinding|GetEstimatedCosttoTarget (LocalVariables|GetinStartIndex) (LocalVariables|GettargetIndex)) (LocalVariables|GetinMovementPoints)))
        (goto _label Break)))
    (:Completed
      (bind _reachabletiles (Pathfinding|FindPathtoTarget (LocalVariables|GetinStartIndex) (LocalVariables|GettargetIndex) true))
      (return _reachabletiles))))

(fn ToggleTacticMode
  (params (bIsTactic :type Boolean))
  (for _array_element (Variables|Default|GetcurrentGridTiles)
    (Default|EventToggleTacticMode _array_element bIsTactic)))