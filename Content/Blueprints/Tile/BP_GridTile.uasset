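; Grid tile actor for a tactical grid that shows terrain difficulty, hover, selection, reachability and path state.
; It reads its data from BP_Grid by index, scales to the grid's tile size and feeds a cost widget.
; Cursor and click events update local flags and notify the grid.
; SetTileColor layers those flags over the terrain color through material parameters, with tactic mode toggling base visibility and the widget.
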(event OnBeginCursorOver(StaticMesh)
  (params (TouchedComponent :type Primitive%20Component%20Object%20Reference))
  ;[1 1 1] Show hover tile
  (CallFunction|EventStartHoverTile)
  (Default|EventNewTileMouseOver (Variables|Grid|Getbp_Grid) self))

(event OnEndCursorOver(StaticMesh)
  (params (TouchedComponent :type Primitive%20Component%20Object%20Reference))
  (Default|EventNewTileMouseOver (Variables|Grid|Getbp_Grid)))

(event OnClicked(StaticMesh)
  (params (TouchedComponent :type Primitive%20Component%20Object%20Reference) (ButtonPressed :type Key%20Structure :default "None"))
  ;[1 1 1] Select Tile on Click
  (CallFunction|EventSelectTile)
  (Default|EventNewTileSelected (Variables|Grid|Getbp_Grid) self))

(event Custom|Event_DeselectTile
  ;[1 1 1] Change color on clicked Tile
  (Variables|Grid|SetbIsSelected false)
  (Grid|SetTileColor))

(event Custom|Event_SelectTile
  ;[1 1 1] Change color on clicked Tile
  (Variables|Grid|SetbIsSelected true)
  (Grid|SetTileColor))

(event Custom|Event_IsReachable
  (params (bIsInPath :type Boolean))
  (Variables|Pathfinding|SetbIsReachable bIsInPath)
  (Grid|SetTileColor))

(event Custom|Event_EndHoverTile
  ;[1 1 1] Change Tile color on Hover
  (Variables|Grid|SetbIsMouseOver false)
  (Grid|SetTileColor))

(event Custom|Event_StartHoverTile
  ;[1 1 1] Change Tile color on Hover
  (Variables|Grid|SetbIsMouseOver true)
  (Grid|SetTileColor))

(event Custom|Event_IsInPath
  (params (bIsInPath :type Boolean))
  ;[1 1 1] If tile is in path to end, change color
  (Variables|Pathfinding|SetbIsInPath bIsInPath)
  (Grid|SetTileColor))

(event Custom|Event_ToggleTacticMode
  (params (bIsTactic :type Boolean))
  (Variables|Default|SetbIsTactic bIsTactic)
  (Development|SetHiddeninGame (Variables|Default|GetWidget) (not (Variables|Default|GetbIsTactic)) false)
  (Grid|SetTileColor))

(event EventBeginPlay
  ;[1 1 1 1 14] On Play, Colorize Tiles based on Terrain Difficulty
  (Utilities|FlowControl|Delay 0.2)
  (Grid|SetTileColor)
  ;[1 1 1 1 14] Set Tile Size ( implicit count) based on variable instance editable
  (Grid|SetTileSize)
  ;[1 1 1 1 14] Display the cost of tiles
  (Pathfinding|SetWidgetVariablesShowCost)
  (CallFunction|EventToggleTacticMode false))

(fn ConstructionScript)

(fn SetTileColor
  (Utilities|FlowControl|Sequence
    (:then_0
      (if (Variables|Default|GetbIsTactic)
        (Rendering|Material|SetScalarParameterValueonMaterials (Variables|Default|GetStaticMesh) "bIsVisible" 1.0)
        (else
          (Rendering|Material|SetScalarParameterValueonMaterials (Variables|Default|GetStaticMesh) "bIsVisible" 0.0))))
    (:then_1
      (switch Utilities|FlowControl|Switch|SwitchonEnum_GroundTypes (.groundtype (Grid|GetTileData))
        (:NewEnumerator0
          (LocalVariables|SetTileColor "(R=0.508662,G=0.541667,B=0.476215,A=1.000000)"))
        (:NewEnumerator1
          (LocalVariables|SetTileColor "(R=0.963542,G=0.895448,B=0.124347,A=1.000000)"))
        (:NewEnumerator2
          (LocalVariables|SetTileColor "(R=0.562500,G=0.174123,B=0.056585,A=1.000000)"))
        (:NewEnumerator3
          (LocalVariables|SetTileColor "(R=0.933333,G=0.000000,B=0.040256,A=1.000000)"))
        (:NewEnumerator4
          (LocalVariables|SetTileColor "(R=0.097486,G=0.100000,B=0.090551,A=1.000000)"))))
    (:then_2
      (if (Variables|Grid|GetbIsSelected)
        (Rendering|Material|SetScalarParameterValueonMaterials (Variables|Default|GetStaticMesh) "bIsSelected" 1.0)
        (Rendering|Material|SetScalarParameterValueonMaterials (Variables|Default|GetStaticMesh) "bIsVisible" 1.0)
        (else
          (Rendering|Material|SetScalarParameterValueonMaterials (Variables|Default|GetStaticMesh) "bIsSelected" 0.0))))
    (:then_3
      (if (Variables|Grid|GetbIsMouseOver)
        (LocalVariables|SettileColor (Math|Conversions|ToLinearColor(Vector) (* (Math|Conversions|ToVector(LinearColor) (LocalVariables|GettileColor)) 3.0)))
        (Rendering|Material|SetScalarParameterValueonMaterials (Variables|Default|GetStaticMesh) "bIsVisible" 1.0)))
    (:then_4
      (if (Variables|Pathfinding|GetbIsReachable)
        (LocalVariables|SetTileColor "(R=0.018739,G=0.384459,B=0.562500,A=1.000000)")
        (Rendering|Material|SetScalarParameterValueonMaterials (Variables|Default|GetStaticMesh) "bIsVisible" 1.0)))
    (:then_5
      (if (Variables|Pathfinding|GetbIsInPath)
        (LocalVariables|SetTileColor "(R=0.066532,G=0.204055,B=1.000000,A=1.000000)")
        (Rendering|Material|SetScalarParameterValueonMaterials (Variables|Default|GetStaticMesh) "bIsVisible" 1.0)))
    (:then_6
      ;[1 1 1] Must be always last, why ?
      (Rendering|Material|SetVectorParameterValueonMaterials (Variables|Default|GetStaticMesh) "TileColor" (Math|Conversions|ToVector(LinearColor) (LocalVariables|GettileColor))))))

(fn GetTileData
  (return (.Value (Utilities|Map|Find (Variables|/Game/Blueprints/BP_Grid.BP_Grid_C|Getstruct_Tiles (Variables|Grid|Getbp_Grid)) (Variables|Grid|GetgridIndex)))))

(fn SetTileSize
  (bind _bp_grid (Variables|Grid|Getbp_Grid))
  (bind _staticmesh (Variables|Default|GetStaticMesh))
  (bind _returnvalue (Transformation|GetWorldScale _staticmesh))
  (bind _tilesize (Variables|/Game/Blueprints/BP_Grid.BP_Grid_C|GetTileSize _bp_grid))
  (bind _returnvalue_2 (/ _tilesize 5e+01))
  (bind _returnvalue_3 (* _returnvalue _returnvalue_2))
  (Transformation|SetWorldScale3D _staticmesh (Math|Vector|MakeVector (.x _returnvalue_3) (.y _returnvalue_3) 1.0)))

(fn SetWidgetVariablesShowCost
  (bind _widget (Variables|Default|GetWidget))
  (bind _returnvalue (UserInterface|GetUserWidgetObject _widget))
  (bind _asw_grid_tile (Utilities|Casting|CastToW_GridTile _returnvalue))
  (Variables|/Game/Blueprints/UI/W_GridTile.W_GridTile_C|Setgrid _asw_grid_tile (Variables|Grid|Getbp_Grid))
  (Variables|/Game/Blueprints/UI/W_GridTile.W_GridTile_C|SetgridIndex _asw_grid_tile (Variables|Grid|GetgridIndex)))