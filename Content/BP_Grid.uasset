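; BP_Grid is a tile grid actor that classifies terrain and previews it with debug drawing from its Construction Script.
; It outlines the grid around the scene component's location, then walks tiles from the bottom-left corner along its right and forward vectors.
; Sphere traces on two channels keep tiles over ground and detect obstacles.
; Each kept tile becomes a colored debug plane, using the obstacle's BP_Base_Obstacle ground type or Normal otherwise.
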(event EventBeginPlay)

(event Collision|EventActorBeginOverlap
  (params (OtherActor :type Actor%20Object%20Reference)))

(event EventTick
  (params (DeltaSeconds :type Float%20%28single-precision%29)))

(fn ConstructionScript
  (bind _gridsizeworld (Variables|Grid|GetGridSizeWorld))
  ;[1 1 1 1 14] Setting Grid World Location at Runtime ( no need to drop anything in the scene then) #1
  (Rendering|Debug|FlushPersistentDebugLines)
  (Variables|Grid|SetGridLocation (Transformation|GetWorldLocation (Variables|Default|GetScene)))
  ;[1 1 1 1 14] Debug the grid outlines ( draw so it is visible) #2
  (Rendering|Debug|DrawDebugBox (Variables|Grid|GetGridLocation) (Math|Vector|MakeVector (.y _gridsizeworld) (.x _gridsizeworld) 5.0) (Variables|Debug|GetGridBoxColor) "0, 0, 0" 5e+03 1e+01)
  ;[1 1 1 1 14] Debug bottom left corner starting point #3 (GridBottomLeft needs to be created first)
  (Rendering|Debug|DrawDebugBox (CallFunction|GridBottomLeft) (Math|Vector|MakeVector 2e+01 2e+01 2e+01) (Variables|Debug|GetBottomLeftColor) "0, 0, 0" 5e+03 1e+01)
  ;[1 1 1 1 14] Draw the Tiles #4 (create DrawTile function beforehand)
  (CallFunction|DrawTile))

(fn GridBottomLeft
  (bind _scene (Variables|Default|GetScene))
  ;[1 1 1 1 14] (Grid Location - ( Scene.GetRightVector * GridSizeX)) - Scene.GetForwardVector * GridSizeY = GridBottomLeft
  (return (- (- (Variables|Grid|GetGridLocation) (* (Math|Vector|GetRightVector _scene) (.x (Variables|Grid|GetGridSizeWorld)))) (* (Math|Vector|GetForwardVector _scene) (.y (Variables|Grid|GetGridSizeWorld))))))

(fn GridTileNumber
  (bind _gridsizeworld (Variables|Grid|GetGridSizeWorld))
  (bind _tilesize (Variables|Grid|GetTileSize))
  (bind _returnvalue (/ _gridsizeworld _tilesize))
  ;[1 1 1 1 14] GridSizeWorld / TileSize. Return (X rounded -1 , Y rounded -1)
  (return (- (Math|Float|Round (.x _returnvalue)) 1) (- (Math|Float|Round (.y _returnvalue)) 1)))

(fn DrawTile
  (bind (_gridtilenumberx _gridtilenumbery) (CallFunction|GridTileNumber))
  (bind _tilesize (Variables|Grid|GetTileSize))
  (bind _tilesize_2 (Variables|Grid|GetTileSize))
  ;[1 1 1 1 14] for x number of tiles, and y number of tiles, x[i] =x , y[j] =y locally saved variables   #part1
  (for _index (range 0 _gridtilenumberx)
    (LocalVariables|SetX _index)
    (for _index_2 (range 0 _gridtilenumbery)
      (LocalVariables|SetY _index_2)
      ;[1 1 1] TilePosition = GridBottomLeft + ( Scene.Right * TileSize) + (Scene.Forward *TileSize), #part2
      ; So it draws a square starting from bottom left position.
      (LocalVariables|SetTilePosition (+ (CallFunction|GridBottomLeft) (* (Math|Vector|GetRightVector (Variables|Default|GetScene)) (+ (* (LocalVariables|GetX) (* _tilesize_2 2.0)) _tilesize_2)) (* (Math|Vector|GetForwardVector (Variables|Default|GetScene)) (+ (* (LocalVariables|GetY) (* _tilesize 2.0)) _tilesize))))
      ;[1 1 1 1 14] Sphere Trace Collision for GROUND, #part4
      (if (.HitSomething (CallFunction|MySphereTrace (LocalVariables|GetTilePosition) "TraceTypeQuery3"))
        ;[1 1 1 1 14] Sphere Trace Collision for OBSTACLES, #part5
        (if (.HitSomething (CallFunction|MySphereTrace (LocalVariables|GetTilePosition) "TraceTypeQuery4"))
          ;[1 1 1 1 14] TILES Draw Debug for 3 other types, #part6
          (CallFunction|MyDrawDebugPlane (LocalVariables|GetTilePosition) (Variables|/Game/BP_Base_Obstacle.BP_Base_Obstacle_C|GetEnum_GroundTypes (.AsBP%20Base%20Obstacle (Utilities|Casting|CastToBP_Base_Obstacle (.Actor (CallFunction|MySphereTrace (LocalVariables|GetTilePosition) "TraceTypeQuery4"))))))
          (else
            ;[1 1 1 1 14] Normal Tiles, #part7
            (CallFunction|MyDrawDebugPlane (LocalVariables|GetTilePosition) "NewEnumerator0")))))))

(fn MySphereTrace
  (params (Location :type Vector) (TraceChannel :type ETraceTypeQuery%20Enum :default "TraceTypeQuery1"))
  (bind (_outhit _returnvalue) (Collision|SphereTraceByChannel Location Location (- (Variables|Grid|GetTileSize) (Variables|Debug|GetGapSize)) TraceChannel false 0 (Variables|Debug|GetDraw%20Debug%20Spheres) true "(R=1.000000,G=0.000000,B=0.000000,A=1.000000)" "(R=0.000000,G=1.000000,B=0.000000,A=1.000000)" 2e+01))
  (return _returnvalue (.hitactor _outhit)))

(fn MyDrawDebugPlane
  (params (Location :type Vector) (GroundType :type Enum_GroundTypes%20Enum :default "NewEnumerator0"))
  (switch Utilities|FlowControl|Switch|SwitchonEnum_GroundTypes GroundType
    (:NewEnumerator0
      (LocalVariables|SetTileColor "(R=0.508662,G=0.541667,B=0.476215,A=1.000000)"))
    (:NewEnumerator1
      (LocalVariables|SetTileColor "(R=0.963542,G=0.895448,B=0.124347,A=1.000000)"))
    (:NewEnumerator2
      (LocalVariables|SetTileColor "(R=0.562500,G=0.174123,B=0.056585,A=1.000000)"))
    (:NewEnumerator3
      (LocalVariables|SetTileColor "(R=0.933333,G=0.000000,B=0.040256,A=1.000000)")))
  (Class|KismetSystemLibrary|DrawDebugPlane (Utilities|Struct|MakePlane (.Z (Math|Vector|BreakVector Location)) 0.0 0.0 1.0) Location (- (Variables|Grid|GetTileSize) (Variables|Debug|GetGapSize)) (LocalVariables|GetTileColor) 1e+06))